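; Bullet_BP is a bullet actor that damages whatever it hits through that actor's HealthSystem component.
; On a Collision hit it toggles its particle system, after checking that the HitComponent's class (not OtherActor's) is not a Bullet_BP child.
; If the other actor has a HealthSystem, it passes Damage to ReceiveDamage, hides the sphere and waits briefly.
; The bullet then destroys itself, immediately when no HealthSystem is found.
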(event `self.Collision.OnComponentHit`
  (params (HitComponent :type "PrimitiveComponent Object Reference") (OtherActor :type "Actor Object Reference") (OtherComp :type "PrimitiveComponent Object Reference") (NormalImpulse :type "Vector Structure") (Hit :type "HitResult Structure (by ref)"))
  (bind _returnvalue (`self.GetComponentByClass` OtherActor "/Game/Alcaval/HealthSystem/HealthSystem.HealthSystem_C"))
  ;[1 1 1] Bullet Component hit behaviour
  (if (not (`KismetMathLibrary.ClassIsChildOf` (`GameplayStatics.GetObjectClass` HitComponent) "Bullet_BP_C"))
    (`ActorComponent.ToggleActive` (`self.ParticleSystem`))
    (if (`KismetSystemLibrary.IsValid` _returnvalue)
      (`/Game/Alcaval/HealthSystem/HealthSystem.receiveDamage` _returnvalue (`self.Damage`))
      (`SceneComponent.ToggleVisibility` (`self.Sphere`) false)
      (`KismetSystemLibrary.Delay` 0.4))
    (`self.K2_DestroyActor`)))

(fn `UserConstructionScript`)