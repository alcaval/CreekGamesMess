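; Player Blueprint that handles automatic shooting while the Shoot input is held.
; Pressing and releasing Shoot sets and clears the IsHolding flag.
; Tick runs through a Delay of ShootRate, which ignores re-triggers while pending and so acts as the fire-rate timer.
; When the delay completes with IsHolding true, it spawns a Bullet_BP at the SpawnProjectile component's world transform.
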(event `self.ReceiveTick`
  (params (DeltaSeconds :type "Float (single-precision)"))
  ;[1 1 1] Shoot system
  (`KismetSystemLibrary.Delay` (`self.ShootRate`))
  (if (`self.isHolding`)
    (`|SpawnActorFromClass` "/Game/Alcaval/Bullet/Bullet_BP.Bullet_BP_C" (`SceneComponent.K2_GetComponentToWorld` (`self.Spawn_Projectile`)) "Undefined" "OverrideRootScale" null null)))

(event `InputAction|Shoot`
  (params (Key :type "Key Structure"))
  ;[1 1 1] Shoot system
  (:`Pressed`
    (set `self.isHolding` true))
  (:`Released`
    (set `self.isHolding` false)))

(fn `UserConstructionScript`
  (`parent.UserConstructionScript`))